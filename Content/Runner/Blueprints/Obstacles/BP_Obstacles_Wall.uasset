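; BP_Obstacles_Wall is a wall obstacle for the runner game that penalizes the player character on overlap.
; Tick uses a one-second Delay to count Timer up roughly once a second, gating overlaps with a short cooldown.
; A valid hit resets Timer, calls Collision on BP_RunnerCharacter, then after a delay sets its max walk speed.
; An unconnected chain for Death and pausing the game never runs.
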(event EventBeginPlay
  (|CallParentFunction))

(event EventTick
  (params (DeltaSeconds :type Float%20%28single-precision%29))
  (|CallParentFunction DeltaSeconds)
  (Utilities|FlowControl|Delay 1.0)
  (Variables|Default|Settimer (+ (Variables|Default|Gettimer) 1.0)))

(event Collision|EventActorBeginOverlap
  (params (OtherActor :type Actor%20Object%20Reference))
  (if (> (Variables|Default|Gettimer) 2.0)
    (Variables|Default|Settimer 0.0)
    (bind _asbp_runner_character (Utilities|Casting|CastToBP_RunnerCharacter OtherActor))
    (Default|Collision _asbp_runner_character)
    (Utilities|FlowControl|Delay 1.0)
    (Variables|/Script/Engine.CharacterMovementComponent|SetMaxWalkSpeed (Variables|/Script/Engine.Character|GetCharacterMovement _asbp_runner_character) 7e+02)))

(fn ConstructionScript
  (|CallParentFunction))
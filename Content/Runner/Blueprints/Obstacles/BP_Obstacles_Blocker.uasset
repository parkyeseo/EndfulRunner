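; Blocker obstacle for the runner game that penalizes a BP_RunnerCharacter overlapping it without sliding.
; A hit calls the character's Collision, then sets its max walk speed to 700 after a one-second delay.
; A Timer, raised about once per second by a Delay on Tick, gates overlaps as a cooldown and resets before the character cast.
; An unconnected death-and-pause chain never runs.
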(event EventBeginPlay
  (|CallParentFunction) ; 지금 이 노드는 비활성 상태입니다. \n핀을 끌어서 다른 노드를 연결하면 활성화됩니다.
)

(event Collision|EventActorBeginOverlap
  (params (OtherActor :type Actor%20Object%20Reference))
  (if (> (Variables|Default|Gettimer) 2.0)
    (Variables|Default|Settimer 0.0)
    (bind _asbp_runner_character (Utilities|Casting|CastToBP_RunnerCharacter OtherActor))
    (if (not (Variables|/Game/Runner/Blueprints/BP_RunnerCharacter.BP_RunnerCharacter_C|GetIs%20Sliding _asbp_runner_character))
      (Default|Collision _asbp_runner_character)
      (Utilities|FlowControl|Delay 1.0)
      (Variables|/Script/Engine.CharacterMovementComponent|SetMaxWalkSpeed (Variables|/Script/Engine.Character|GetCharacterMovement _asbp_runner_character) 7e+02))))

(event EventTick
  (params (DeltaSeconds :type Float%20%28single-precision%29))
  (|CallParentFunction DeltaSeconds)
  (Utilities|FlowControl|Delay 1.0)
  (Variables|Default|Settimer (+ (Variables|Default|Gettimer) 1.0)))

(fn ConstructionScript
  (|CallParentFunction))